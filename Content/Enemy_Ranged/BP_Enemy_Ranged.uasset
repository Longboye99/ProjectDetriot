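; Ranged enemy character Blueprint that holds a weapon, takes damage and dies.
; On BeginPlay it snaps the Weapon component to the mesh's Hand_R socket.
; AnyDamage prints a debug message and subtracts from Health while it is positive, calling Die to destroy the actor at zero or below.
; A SetWalkSpeed function sets the movement speed; the graphs shown contain no attack logic.
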(event `self.ReceiveBeginPlay`
  (`SceneComponent.K2_AttachToComponent` (`self.Weapon`) (`self.Mesh`) "Hand_R" "SnapToTarget" "SnapToTarget" "SnapToTarget" true))

(event `self.ReceiveAnyDamage`
  (params (Damage :type "Float (single-precision)") (DamageType :type "DamageType Object Reference") (InstigatedBy :type "Controller Object Reference") (DamageCauser :type "Actor Object Reference"))
  (bind _health (`self.Health`))
  (`KismetSystemLibrary.PrintString` "Damaged")
  (if (> _health 0.0)
    (bind _output_get (set `self.Health` (- _health Damage)))
    (if (<= _output_get 0.0)
      (`self.Die`))))

(event `Die`
  (`self.K2_DestroyActor`))

(fn `SetWalkSpeed`
  (params (Speed :type "Float (double-precision)"))
  (set `CharacterMovementComponent.MaxWalkSpeed` Speed (`self.CharacterMovement`)))

(fn `UserConstructionScript`)