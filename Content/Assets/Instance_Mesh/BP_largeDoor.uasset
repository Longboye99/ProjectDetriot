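; Blueprint for a large double sliding door that opens when something overlaps its trigger box and closes when the overlap ends.
; A Door_Control timeline plays forward on begin overlap and reverses on end overlap.
; Its track drives a vector lerp that moves the right and left panels between a shared closed position and separate open offsets.
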(event `self.Box.OnComponentBeginOverlap`
  (params (OverlappedComponent :type "PrimitiveComponent Object Reference") (OtherActor :type "Actor Object Reference") (OtherComp :type "PrimitiveComponent Object Reference") (OtherBodyIndex :type Integer) (bFromSweep :type Boolean) (SweepResult :type "HitResult Structure (by ref)"))
  (bind (_direction _newtrack_0) (`Timeline|Door_Control` :!label _label)
    (:`Update`
      (`SceneComponent.K2_SetRelativeLocation` (`self.D_R`) (`KismetMathLibrary.VLerp` (`self.DoorClose`) (`self.DoorOpenR`) _newtrack_0) false false)
      (`SceneComponent.K2_SetRelativeLocation` (`self.D_L`) (`KismetMathLibrary.VLerp` (`self.DoorClose`) (`self.DoorOpenL`) _newtrack_0) false false))))

(event `self.Box.OnComponentEndOverlap`
  (params (OverlappedComponent :type "PrimitiveComponent Object Reference") (OtherActor :type "Actor Object Reference") (OtherComp :type "PrimitiveComponent Object Reference") (OtherBodyIndex :type Integer))
  (goto _label :!via `Reverse`))

(fn `UserConstructionScript`)