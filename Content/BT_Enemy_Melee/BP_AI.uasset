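; BP_AI is a melee enemy character that detects, punches and can be killed by the player, BP_FPShooter.
; PawnSensing sets a blackboard flag when it sees the player.
; AttackPlayer sphere-traces ahead and, on hitting the player, plays a punch montage, applies damage and plays a sound.
; Incoming damage drains HP until Die disables capsule collision, stops movement, ragdolls the mesh and destroys the actor after a delay.
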(event `self.PawnSensing.OnSeePawn`
  (params (Pawn :type "Pawn Object Reference"))
  (cast `/Game/Variant_Shooter/Blueprints/FirstPerson/BP_FPShooter` Pawn)
  (`BlackboardComponent.SetValueAsBool` (`AIBlueprintHelperLibrary.GetBlackboard` (`AIBlueprintHelperLibrary.GetAIController` self)) "hasSeenPlayer?" true))

(event `Attack Player`
  (bind _returnvalue (`self.K2_GetActorLocation`))
  (if (not (`self.Dying`))
    (bind (_outhit _returnvalue_2) (`KismetSystemLibrary.SphereTraceSingleForObjects` :`Start` _returnvalue :`End` (+ _returnvalue (* (`KismetMathLibrary.GetForwardVector` (`self.K2_GetActorRotation`)) 250.0)) :`Radius` 120.0 :`ObjectTypes` (`|MakeArray` "ObjectTypeQuery3" :!type "EObjectTypeQuery Enum") :`DrawDebugType` "ForOneFrame"))
    (if _returnvalue_2
      (bind (_bblockinghit _binitialoverlap _time _distance _location _impactpoint _normal _impactnormal _physmat _hitactor) (`GameplayStatics.BreakHitResult` _outhit))
      (cast `/Game/Variant_Shooter/Blueprints/FirstPerson/BP_FPShooter` _hitactor)
      (`self.PlayAnimMontage` "/Game/BT_Enemy_Melee/Mixamo/Exo_Red/Punching_Anim_Montage.Punching_Anim_Montage")
      (`GameplayStatics.ApplyDamage` _hitactor 10.0)
      (`GameplayStatics.PlaySoundAtLocation` "/Game/Sound/WeaponSound/Cyber_Punch_-_Sound_Effect__HQ_.Cyber_Punch_-_Sound_Effect__HQ_" _location (struct) 0.6 1.0 0.0 null null null null))))

(event `self.ReceiveAnyDamage`
  (params (Damage :type "Float (single-precision)") (DamageType :type "DamageType Object Reference") (InstigatedBy :type "Controller Object Reference") (DamageCauser :type "Actor Object Reference"))
  (if (> (`self.Current HP`) 0.0)
    (bind _output_get (set `self.Current HP` (- (`self.Current HP`) Damage)))
    (if (<= _output_get 0.0)
      (`self.Die`))))

(event `Die`
  (bind _mesh (`self.Mesh`))
  (bind _charactermovement (`self.CharacterMovement`))
  (set `self.Dying` true)
  (`/Engine/EditorBlueprintResources/StandardMacros.DoOnce` false
    (:`Completed`
      (`PrimitiveComponent.SetCollisionEnabled` (`self.CapsuleComponent`) "NoCollision")
      (`MovementComponent.StopMovementImmediately` _charactermovement)
      (`NavMovementInterface.StopActiveMovement` _charactermovement)
      (`PrimitiveComponent.SetCollisionProfileName` _mesh "Ragdoll" true)
      (`PrimitiveComponent.SetSimulatePhysics` _mesh true)
      (`SkeletalMeshComponent.SetPhysicsBlendWeight` _mesh 1.0)
      (`KismetSystemLibrary.Delay` 2.0)
      (`self.K2_DestroyActor`))))

(fn `UserConstructionScript`)